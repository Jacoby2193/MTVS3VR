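; VR player pawn that sets up stage tracking and Enhanced Input when an HMD is active, and links itself to the main widget.
; Right-hand triggers drive hand animation alphas, click UI through a widget interaction component, and grab or release physics-driven BP_GrabObject actors at a socket.
; Right thumbstick either teleports along a predicted projectile arc drawn with Niagara or slides in world axes.
; Left-hand inputs only write to a debug log.
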(event Input|EnhancedActionEvents|EnhancedInputActionIA_IndexTrigger_Left
  (params (ActionValue :type Boolean) (ElapsedSeconds :type Float%20%28double-precision%29) (TriggeredSeconds :type Float%20%28double-precision%29) (InputAction :type Input%20Action%20Object%20Reference :default "/Game/Technoise/Inputs/IA_IndexTrigger_Left.IA_IndexTrigger_Left"))
  (bind _leftlog (Variables|Default|GetLeftLog))
  (:Started
    (Rendering|Components|TextRender|SetText _leftlog (Utilities|Text|MakeLiteralText "Index Trigger Pressed!")))
  (:Completed
    (Rendering|Components|TextRender|SetText _leftlog (Utilities|Text|MakeLiteralText "Index Trigger Released!"))))

(event Input|EnhancedActionEvents|EnhancedInputActionIA_HandTrigger_Left
  (params (ActionValue :type Boolean) (ElapsedSeconds :type Float%20%28double-precision%29) (TriggeredSeconds :type Float%20%28double-precision%29) (InputAction :type Input%20Action%20Object%20Reference :default "/Game/Technoise/Inputs/IA_HandTrigger_Left.IA_HandTrigger_Left"))
  (bind _leftlog (Variables|Default|GetLeftLog))
  (:Started
    (Rendering|Components|TextRender|SetText _leftlog (Utilities|Text|MakeLiteralText "Hand Trigger Pressed!")))
  (:Completed
    (Rendering|Components|TextRender|SetText _leftlog (Utilities|Text|MakeLiteralText "Hand Trigger Released!"))))

(event Input|EnhancedActionEvents|EnhancedInputActionIA_ThumbstickAxis_Left
  (params (ActionValue :type Vector%202D%20Structure) (ElapsedSeconds :type Float%20%28double-precision%29) (TriggeredSeconds :type Float%20%28double-precision%29) (InputAction :type Input%20Action%20Object%20Reference :default "/Game/Technoise/Inputs/IA_ThumbstickAxis_Left.IA_ThumbstickAxis_Left"))
  (bind _returnvalue (Utilities|Text|ToText(String) ActionValue))
  (bind _leftlog (Variables|Default|GetLeftLog))
  (:Triggered
    (Rendering|Components|TextRender|SetText _leftlog _returnvalue))
  (:Completed
    (Rendering|Components|TextRender|SetText _leftlog _returnvalue)))

(event Input|EnhancedActionEvents|EnhancedInputActionIA_HandTriggerFloat_Right
  (params (ActionValue :type Float%20%28double-precision%29) (ElapsedSeconds :type Float%20%28double-precision%29) (TriggeredSeconds :type Float%20%28double-precision%29) (InputAction :type Input%20Action%20Object%20Reference :default "/Game/Technoise/Inputs/IA_HandTriggerFloat_Right.IA_HandTriggerFloat_Right"))
  (bind _right_hand_anim (Variables|Default|GetRight%20Hand%20Anim))
  (:Triggered
    (Variables|/Game/Technoise/Animations/ABP_MTVS3Hand.ABP_MTVS3Hand_C|SetPoseAlphaGrasp _right_hand_anim ActionValue))
  (:Completed
    (Variables|/Game/Technoise/Animations/ABP_MTVS3Hand.ABP_MTVS3Hand_C|SetPoseAlphaGrasp _right_hand_anim ActionValue)))

(event Input|EnhancedActionEvents|EnhancedInputActionIA_IndexTriggerFloat_Right
  (params (ActionValue :type Float%20%28double-precision%29) (ElapsedSeconds :type Float%20%28double-precision%29) (TriggeredSeconds :type Float%20%28double-precision%29) (InputAction :type Input%20Action%20Object%20Reference :default "/Game/Technoise/Inputs/IA_IndexTriggerFloat_Right.IA_IndexTriggerFloat_Right"))
  (bind _right_hand_anim (Variables|Default|GetRight%20Hand%20Anim))
  (:Triggered
    (Variables|/Game/Technoise/Animations/ABP_MTVS3Hand.ABP_MTVS3Hand_C|SetPoseAlphaIndexCurl _right_hand_anim ActionValue))
  (:Completed
    (Variables|/Game/Technoise/Animations/ABP_MTVS3Hand.ABP_MTVS3Hand_C|SetPoseAlphaIndexCurl _right_hand_anim ActionValue)))

(event Input|EnhancedActionEvents|EnhancedInputActionIA_HandTrigger_Right
  (params (ActionValue :type Boolean) (ElapsedSeconds :type Float%20%28double-precision%29) (TriggeredSeconds :type Float%20%28double-precision%29) (InputAction :type Input%20Action%20Object%20Reference :default "/Game/Technoise/Inputs/IA_HandTrigger_Right.IA_HandTrigger_Right"))
  (:Started
    (CallFunction|GrabAction))
  (:Completed
    (CallFunction|ReleaseAction)))

(event Input|EnhancedActionEvents|EnhancedInputActionIA_ThumbstickAxis_Right
  (params (ActionValue :type Vector%202D%20Structure) (ElapsedSeconds :type Float%20%28double-precision%29) (TriggeredSeconds :type Float%20%28double-precision%29) (InputAction :type Input%20Action%20Object%20Reference :default "/Game/Technoise/Inputs/IA_ThumbstickAxis_Right.IA_ThumbstickAxis_Right"))
  (bind _use_teleport (Variables|Default|GetUse%20Teleport))
  (:Triggered
    (if _use_teleport
      (CallFunction|DrawTeleportLine)
      (else
        (CallFunction|NormalMove ActionValue))))
  (:Completed
    (if _use_teleport
      (CallFunction|TeleportAction)
      (else
        (CallFunction|NormalMove ActionValue)))))

(event Input|EnhancedActionEvents|EnhancedInputActionIA_IndexTrigger_Right
  (params (ActionValue :type Boolean) (ElapsedSeconds :type Float%20%28double-precision%29) (TriggeredSeconds :type Float%20%28double-precision%29) (InputAction :type Input%20Action%20Object%20Reference :default "/Game/Technoise/Inputs/IA_IndexTrigger_Right.IA_IndexTrigger_Right"))
  (bind _rightwidgetinteractioncomp (Variables|Default|GetRightWidgetInteractionComp))
  (:Started
    (Class|WidgetInteractionComponent|PressPointerKey _rightwidgetinteractioncomp "LeftMouseButton"))
  (:Completed
    (Class|WidgetInteractionComponent|ReleasePointerKey _rightwidgetinteractioncomp "LeftMouseButton")))

(event EventBeginPlay
  (if (Class|HeadMountedDisplayFunctionLibrary|IsHeadMountedDisplayEnabled)
    (Class|HeadMountedDisplayFunctionLibrary|SetTrackingOrigin "Stage")
    (Input|AddMappingContext (PlayerController|LocalPlayerSubsystems|GetEnhancedInputLocalPlayerSubsystem (Game|GetPlayerController 0)) "/Game/Technoise/Inputs/IMC_MTVS3InputMappings.IMC_MTVS3InputMappings" 0 "(bIgnoreAllPressedKeysUntilRelease=True,bForceImmediately=False,bNotifyUserSettings=False)")
    (bind _asabp_mtvs3hand (Utilities|Casting|CastToABP_MTVS3Hand (Components|SkeletalMesh|GetAnimInstance (Variables|Default|GetRightHand))))
    (Variables|Default|SetRight%20Hand%20Anim _asabp_mtvs3hand)
    (bind _aswbp_main_widget (Utilities|Casting|CastToWBP_MainWidget (UserInterface|GetWidget (Variables|Default|GetMainWidget))))
    (Variables|/Game/Technoise/UI/WBP_MainWidget.WBP_MainWidget_C|SetPlayer _aswbp_main_widget self)))

(event Collision|EventActorBeginOverlap
  (params (OtherActor :type Actor%20Object%20Reference)))

(event EventTick
  (params (DeltaSeconds :type Float%20%28single-precision%29)))

(fn ConstructionScript)

(fn GrabAction
  (Utilities|IsValid (Variables|Default|GetCurrent%20Grabbed%20Actor)
    (:Is%20Not%20Valid
      (bind _outactors (Collision|SphereOverlapActors (Transformation|GetWorldLocation (Variables|Default|GetRightMotionController)) 0.0 (Utilities|Array|MakeArray "ObjectTypeQuery2") "/Game/Technoise/Blurprints/BP_GrabObject.BP_GrabObject_C" (Utilities|Array|MakeArray self)))
      (bind _asbp_grab_object (Utilities|Casting|CastToBP_GrabObject (Utilities|Array|Get(acopy) _outactors)))
      (Physics|SetSimulatePhysics (Variables|/Game/Technoise/Blurprints/BP_GrabObject.BP_GrabObject_C|GetBox _asbp_grab_object) false)
      (Transformation|AttachComponentToComponent _asbp_grab_object (Variables|Default|GetRightHand) "GrabPoint" "SnapToTarget" "KeepWorld" "KeepWorld" true)
      (Variables|Default|SetCurrent%20Grabbed%20Actor _asbp_grab_object))))

(fn ReleaseAction
  (Utilities|IsValid (Variables|Default|GetCurrent%20Grabbed%20Actor)
    (:Is%20Valid
      (Transformation|DetachFromActor (Variables|Default|GetCurrent%20Grabbed%20Actor) "KeepWorld" "KeepWorld" "KeepWorld")
      (Physics|SetSimulatePhysics (Variables|/Game/Technoise/Blurprints/BP_GrabObject.BP_GrabObject_C|GetBox (Variables|Default|GetCurrent%20Grabbed%20Actor)) true)
      (Variables|Default|SetCurrent%20Grabbed%20Actor 0))))

(fn NormalMove
  (params (InputValue :type Vector%202D%20Structure))
  (Transformation|SetActorLocation (+ (Transformation|GetActorLocation) (* (Math|Vector|Normalize (Math|Vector|MakeVector (.y InputValue) (.x InputValue) 0.0)) 5e+01)) false false))

(fn DrawTeleportLine
  (bind _rightmotioncontroller (Variables|Default|GetRightMotionController))
  (bind _teleportdestination (Variables|Default|GetTeleportDestination))
  (bind (_outhit _outpathpositions _outlasttracedestination) (Class|GameplayStatics|BlueprintPredictProjectilePathbyTraceChannel (Transformation|GetWorldLocation _rightmotioncontroller) (* (Math|Vector|GetForwardVector _rightmotioncontroller) (Variables|Default|GetTeleport%20Power)) true 0.0 "ECC_WorldDynamic" false (Utilities|Array|MakeArray self) "None"))
  (Class|NiagaraDataInterfaceArrayFunctionLibrary|SetNiagaraArrayVector (Variables|Default|GetTeleportLine) "PointArray" _outpathpositions)
  (Rendering|SetVisibility _teleportdestination true false)
  (Transformation|SetWorldLocation _teleportdestination _outlasttracedestination false false)
  (Variables|Default|SetDestination%20Location _outlasttracedestination))

(fn TeleportAction
  (Class|NiagaraDataInterfaceArrayFunctionLibrary|SetNiagaraArrayVector (Variables|Default|GetTeleportLine) "PointArray" (Utilities|Array|MakeArray "0, 0, 0"))
  (Rendering|SetVisibility (Variables|Default|GetTeleportDestination) false false)
  (Transformation|SetActorLocation (+ (Variables|Default|GetDestination%20Location) "0.000000,0.000000,50.000000") false false))